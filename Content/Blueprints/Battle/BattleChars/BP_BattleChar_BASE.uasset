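; Base battle character actor that handles attack and knockout animations, defending state, target pointer and battle UI links.
; Initializes shaker and stats components, relaying battle effects between its stats and BattleManager.
; Attacks play the data-defined animation override or fall back to a timeline hop, then notify BattleManager.
; On depleted health it updates team status, hides its portrait, then jumps party members to a downed state or slides others away and hides them.
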(event Custom|PlayAttackAnim
  (bind _spawnedlocation_ (Variables|Default|GetSpawnedLocation%20))
  (bind _attackanimdefault (Variables|/Game/Data/DataAssets/BattleCharData/PDA_BattleCharData.PDA_BattleCharData_C|GetAttackAnimDefault (Variables|Default|GetBattleCharData))
    (:then
      (|PlayAnimationOverridewithCallbacks (Variables|/Script/PaperZD.PaperZDAnimationComponent|GetAnimInstance (Variables|Default|GetAnimationComponent)) _attackanimdefault "DefaultSlot" 1.0 0.0
        (:OnCompleted
          _)
        (:OnCancelled
          _))
      (Utilities|FlowControl|RetriggerableDelay (Variables|Default|GetAfter%20Attack%20Delay))
      (Default|MoveBackfromActive (Variables|Default|GetBattleManager)))
    (:else
      (Components|Timeline|SetPlayRate (Variables|Default|GetAnimDoubleJump) (Variables|Default|GetJumpRate))
      (bind _alpha (Timeline|AnimDoubleJump PlayFromStart)
        (:Update
          (Transformation|SetActorLocation (Math|Vector|MakeVector (.x _spawnedlocation_) (.y _spawnedlocation_) (+ (.z _spawnedlocation_) (* _alpha (Variables|Default|GetJumpHeight)))) false false))
        (:Finished
          (Default|FinishedTimelineAttackAnim (Variables|Default|GetBattleManager)))))))

(event Custom|PlayKOAnim
  (Components|Timeline|SetPlayRate (Variables|Default|GetAnimKO) (Variables|Default|GetKnockoutAnimPlayRate))
  (bind _alpha (Timeline|AnimKO PlayFromStart)
    (:Update
      (Transformation|SetActorLocation (Math|Vector|Lerp(Vector) (Variables|Default|GetSpawnedLocation%20) (+ (Variables|Default|GetSpawnedLocation%20) (Variables|Default|GetKnockoutOffset)) _alpha) false false))
    (:Finished
      (Rendering|SetActorHiddenInGame true))))

(event EventBeginPlay
  (Utilities|FlowControl|Sequence
    (:then_0
      (Variables|Default|SetSpawnedLocation%20 (Transformation|GetActorLocation))
      (bind _aswbp_target_pointer (Utilities|Casting|CastToWBP_TargetPointer (UserInterface|GetUserWidgetObject (Variables|Default|GetWidgetPointer))))
      (Variables|Default|SetWidgetTargetPointer _aswbp_target_pointer))
    (:then_1
      (Default|Initialize (Variables|Default|GetAC_Shaker) (Variables|Default|GetSprite))
      (Default|Initialize (Variables|Default|GetAC_BattleStats) self))))

(event Collision|EventActorBeginOverlap
  (params (OtherActor :type Actor%20Object%20Reference)))

(event EventTick
  (params (DeltaSeconds :type Float%20%28single-precision%29)))

(fn ConstructionScript)

(fn HideBattlePortrait
  (bind _widgetportrait (Variables|Default|GetWidgetPortrait)
    (:then
      (Default|HidePortrait _widgetportrait)
      (Variables|Default|SetWidgetPortrait 0))
    (:else)))

(fn AssignBattleHealthManaWidget
  (params (WidgetHealthMana :type WBP%20Battle%20Health%20Mana%20Object%20Reference))
  (bind _ac_battlestats (Variables|Default|GetAC_BattleStats))
  (bind _ac_battlestats_2 (Variables|Default|GetAC_BattleStats))
  (bind _attributes (Variables|/Game/Blueprints/Components/AC_BattleStats.AC_BattleStats_C|GetAttributes _ac_battlestats_2))
  (bind _state (Variables|/Game/Blueprints/Components/AC_BattleStats.AC_BattleStats_C|GetState _ac_battlestats))
  (bind (_maxhp _maxmp) (Utilities|Struct|BreakS_CharAttributes _attributes))
  (bind (_hp _mp) (Utilities|Struct|BreakS_CharState _state))
  (Variables|Default|SetWidgetHealthMana WidgetHealthMana)
  (Default|Activate (Variables|Default|GetWidgetHealthMana) (Variables|/Game/Data/DataAssets/BattleCharData/PDA_BattleCharData.PDA_BattleCharData_C|GetDisplayName (Variables|Default|GetBattleCharData)) _maxhp _hp _maxmp _mp))

(fn SetPointerVisibility
  (params (SetVisible :type Boolean))
  (if SetVisible
    (Default|ShowPointer (Variables|Default|GetWidgetTargetPointer))
    (else
      (Default|HidePointer (Variables|Default|GetWidgetTargetPointer)))))

(fn RecivedBattleEffect
  (params (InstigatorStats :type AC%20Battle%20Stats%20Object%20Reference))
  (Default|RecieveBattleEffect (Variables|Default|GetAC_BattleStats) InstigatorStats))

(fn ExecuteBattleEffect
  (Default|ApplyBattleEffect (Variables|Default|GetBattleManager) (Variables|Default|GetAC_BattleStats)))

(fn SetDefending
  (params (SetActive :type Boolean))
  (Variables|Default|SetIsDefending SetActive))

(fn DepletedHealth
  (Utilities|FlowControl|Sequence
    (:then_0
      (Default|UpdateTeamAlive (Variables|Default|GetBattleManager) self)
      (bind _widgetportrait (Variables|Default|GetWidgetPortrait)
        (:then
          (Default|HidePortrait _widgetportrait))
        (:else)))
    (:then_1
      ;[0.15 0.15 0.15 0.5] Failsafe Logic
      (if (Variables|Default|GetIsPartyMember)
        (Class|PaperZDAnimInstance|JumptoNode (Variables|/Script/PaperZD.PaperZDAnimationComponent|GetAnimInstance (Variables|Default|GetAnimationComponent)) "JumpDowned" "None")
        (else
          (CallFunction|PlayKOAnim))))))