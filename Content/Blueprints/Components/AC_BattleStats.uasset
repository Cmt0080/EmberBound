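; Battle stats component that holds a combatant's attributes and HP/MP state, initialized from its character data.
; Incoming skills compute power and crit from the instigator's stats, then apply defense reduction and the Defend multiplier, with at least 1 damage.
; The result updates HP, the health widget and combat numbers, then triggers knockout at zero HP or a hit shake otherwise.
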(event EventBeginPlay)

(event EventTick
  (params (DeltaSeconds :type Float%20%28single-precision%29)))

(fn Initialize
  (params (OwningBattleChar :type BP%20Battle%20Char%20BASE%20Object%20Reference))
  (Variables|Default|SetOwningBattleChar OwningBattleChar)
  (Variables|Default|SetAttributes (Variables|/Game/Data/DataAssets/BattleCharData/PDA_BattleCharData.PDA_BattleCharData_C|GetInitalAttributes (Variables|/Game/Blueprints/Battle/BattleChars/BP_BattleChar_BASE.BP_BattleChar_BASE_C|GetBattleCharData (Variables|Default|GetOwningBattleChar))))
  (Utilities|Struct|SetmembersinS_CharState (Variables|Default|GetState) (.MaxHp (Utilities|Struct|BreakS_CharAttributes (Variables|Default|GetAttributes))) (.MaxMP (Utilities|Struct|BreakS_CharAttributes (Variables|Default|GetAttributes)))))

(fn RecieveBattleEffect
  (params (InstigatorStats :type AC%20Battle%20Stats%20Object%20Reference) (SkillData :type PDA%20Skill%20Data%20Object%20Reference))
  (Utilities|FlowControl|Sequence
    (:then_0
      (bind (_calculatedpower _wascritical) (Default|GetCalculatedPower SkillData InstigatorStats))
      (LocalVariables|SetIsCritical _wascritical)
      (bind _damage (CallFunction|DamageAfterDefense _calculatedpower (Variables|/Game/Data/DataAssets/SkillData/PDA_SkillData.PDA_SkillData_C|GetisPhysical SkillData)))
      (LocalVariables|SetFinalValue (Math|Conversions|ToFloat(Integer) (Math|Integer|Max(Integer) (Math|Float|Round _damage) 1)))
      (Utilities|Struct|SetmembersinS_CharState (Variables|Default|GetState) (Math|Float|Max(Float) (- (Utilities|Struct|BreakS_CharState (Variables|Default|GetState)) (LocalVariables|GetFinalValue)) 0.0))
      (bind _widgethealthmana (Variables|/Game/Blueprints/Battle/BattleChars/BP_BattleChar_BASE.BP_BattleChar_BASE_C|GetWidgetHealthMana (Variables|Default|GetOwningBattleChar))
        (:then
          (Default|UpdateHP _widgethealthmana (Utilities|Struct|BreakS_CharState (Variables|Default|GetState)) (Utilities|Struct|BreakS_CharAttributes (Variables|Default|GetAttributes))))
        (:else)))
    (:then_1
      (Default|ShowText (Variables|/Game/Blueprints/Battle/BattleChars/BP_BattleChar_BASE.BP_BattleChar_BASE_C|GetWidgetCombatNumber (Variables|Default|GetOwningBattleChar)) (LocalVariables|GetFinalValue) (select (LocalVariables|GetIsCritical) "NewEnumerator1" "NewEnumerator0")))
    (:then_2
      (if (<= (Utilities|Struct|BreakS_CharState (Variables|Default|GetState)) 0.0)
        (Utilities|Struct|SetmembersinS_CharState (Variables|Default|GetState) true)
        (Default|DepletedHealth (Variables|Default|GetOwningBattleChar))
        (else
          (Default|StartShake (Variables|/Game/Blueprints/Battle/BattleChars/BP_BattleChar_BASE.BP_BattleChar_BASE_C|GetAC_Shaker (Variables|Default|GetOwningBattleChar))))))))

(fn DamageAfterDefense
  (params (IncomingDamage :type Float%20%28double-precision%29) (IsPhysical :type Boolean))
  (return (* (- IncomingDamage (|DamageReduction)) (select (Variables|/Game/Blueprints/Battle/BattleChars/BP_BattleChar_BASE.BP_BattleChar_BASE_C|GetIsDefending (Variables|Default|GetOwningBattleChar)) (Variables|/Game/Data/DataAssets/GlobalVariables/PDA_GlobalVariables.PDA_GlobalVariables_C|GetDefendMultiplier (CallFunction|GetGlobalVariables)) 1.0))))