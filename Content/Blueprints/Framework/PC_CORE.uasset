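; PC_CORE is the core player controller, handling creation of the field and battle HUD widgets and switching between game and UI input.
; Interface events create WBP_Field or WBP_Battle, store the reference and add it to the viewport, while interface getters return those references to callers.
; Other interface events toggle UI-only input focused on a given widget or game-only input, showing or hiding the mouse cursor to match.
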(event EventBeginPlay)

(event EventTick
  (params (DeltaSeconds :type Float%20%28single-precision%29)))

(event EventIInitWidgetField
  (CallFunction|InitWidgetField))

(event EventIInitWidgetBattle
  (CallFunction|InitWidgetBattle))

(event EventIActivateUIControls
  (params (WidgetToFocus :type Widget%20Object%20Reference))
  (CallFunction|ActivateUIControls WidgetToFocus))

(event EventIDeactivateUIControls
  (CallFunction|DeactivateUIControls))

(fn ConstructionScript)

(fn InitWidgetBattle
  (bind _returnvalue (UserInterface|CreateWidget "/Game/UI/Widgets/WBP_Battle.WBP_Battle_C" self))
  (bind _output_get (Variables|Default|SetWidgetBattle _returnvalue))
  (UserInterface|Viewport|AddtoViewport _output_get 0))

(fn InitWidgetField
  (bind _returnvalue (UserInterface|CreateWidget "/Game/UI/Widgets/WBP_Field.WBP_Field_C" self))
  (bind _output_get (Variables|Default|SetWidgetField _returnvalue))
  (UserInterface|Viewport|AddtoViewport _output_get 0))

(fn NewFunction)

(fn ActivateUIControls
  (params (InWidgetToFocus :type Widget%20Object%20Reference))
  (Input|SetInputModeUIOnly (Game|GetPlayerController 0) InWidgetToFocus "DoNotLock" true)
  (Variables|/Script/Engine.PlayerController|SetbShowMouseCursor (Game|GetPlayerController 0) true))

(fn DeactivateUIControls
  (Input|SetInputModeGameOnly (Game|GetPlayerController 0) true)
  (Variables|/Script/Engine.PlayerController|SetbShowMouseCursor (Game|GetPlayerController 0) false))

(fn IGetWidgetBattle
  (return (Variables|Default|GetWidgetBattle)))

(fn IGetWidgetField
  (return (Variables|Default|GetWidgetField)))